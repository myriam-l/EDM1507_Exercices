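; MIDI manager Blueprint that plays the MSS_Polysynth sound from an external MIDI controller.
; On BeginPlay it opens the input device matching MidiControlerIndex and binds its MIDI events.
; Note On spawns a 2D sound stored in PolyVoices by note number; Note Off triggers that voice's release.
; Control Change handling is unfinished, with an unnamed parameter; MonoSynth knob mappings are left disconnected.
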(event Custom|EventOnMIDIEvent
  (params (MIDIDeviceController :type MIDI%20Device%20Controller%20Object%20Reference) (Timestamp :type Integer) (EventType :type EMIDIEventType%20Enum :default "Unknown") (Channel :type Integer) (ControlID :type Integer) (Velocity :type Integer) (RawEventType :type Integer))
  (bind _returnvalue (Math|Conversions|ToFloat(Integer) ControlID))
  (bind _returnvalue_2 (Math|Float|Truncate _returnvalue))
  (Development|PrintString (Utilities|String|ToString(Text) (Utilities|Text|FormatText "MIDINOTE{note}VELOCITE{velocite}event{event}" ControlID Velocity (Utilities|String|EnumtoString EventType))) true true "(R=0.000000,G=0.660000,B=1.000000,A=1.000000)" 2.0 "MIDI")
  (switch Utilities|FlowControl|Switch|SwitchonEMIDIEventType EventType
    (:NoteOff
      ;[0.15 0.15 0.15 0.5] ce que ca faiit quand on lache la note
      (Class|AudioParameterControllerInterface|SetTriggerParameter (Utilities|Array|Get(acopy) (Variables|Default|GetPolyVoices) (Math|Float|Truncate _returnvalue)) "Trigger Release"))
    (:NoteOn
      ;[0.15 0.15 0.15 0.5] ce que ca fait quand je clic sur la note
      (bind _returnvalue_3 (Audio|CreateSound2D "/Game/Metasound/MSS_Polysynth.MSS_Polysynth" 1.0 1.0 0.0 0))
      (Utilities|Array|SetArrayElem (Variables|Default|GetPolyVoices) _returnvalue_2 _returnvalue_3 true)
      (Audio|Parameter|SetFloatParameter _returnvalue_3 "MidiNote" _returnvalue :!class /Script/AudioExtensions.AudioParameterControllerInterface)
      (Audio|Components|Audio|Play _returnvalue_3 0.0))
    (:ControlChange
      (switch string (Utilities|String|ToString(Integer) _returnvalue_2)
        (:74
          (for _array_element (Variables|Default|GetPolyVoices)
            (Utilities|IsValid _array_element
              (:Is%20Valid
                (Audio|Parameter|SetFloatParameter _array_element "None" (Math|Conversions|ToFloat(Integer) (/ 127 ControlID)) :!class /Script/Engine.AudioComponent)))))))))

(event EventBeginPlay
  (bind _outmididevices (Class|MIDIDeviceManager|FindMIDIDevices))
  (for _array_element _outmididevices
    (if (.bCanReceiveFrom (Utilities|Struct|BreakFoundMIDIDevice _array_element))
      (if (== (Variables|Default|GetMidi%20controler%20index) (.DeviceID (Utilities|Struct|BreakFoundMIDIDevice _array_element)))
        (Development|PrintString (Utilities|String|ToString(Integer) (.DeviceID (Utilities|Struct|BreakFoundMIDIDevice _array_element))))
        (bind _returnvalue (Class|MIDIDeviceManager|CreateMIDIDeviceController (.DeviceID (Utilities|Struct|BreakFoundMIDIDevice _array_element)) 1024))
        ;[0.15 0.15 0.15 0.5] promote to variable
        (bind _output_get (Variables|Default|SetMidi%20controle _returnvalue))
        (EventDispatchers|BindEventtoOnMIDIEvent _output_get (EventDispatchers|CreateEvent :!event EventonMIDIEvent)))))
  (Development|PrintString "boucle terminée" true true "(R=0.000000,G=0.660000,B=1.000000,A=1.000000)" 3e+01))

(fn ConstructionScript)